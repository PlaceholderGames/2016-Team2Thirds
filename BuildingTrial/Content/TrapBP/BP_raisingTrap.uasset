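; BP_raisingTrap is a one-shot cage trap that moves when its actor is overlapped and briefly immobilises the player.
; On overlap it stores the cage's location and, once only, zeroes the player character's walk speed and plays the TrapFalling timeline.
; Timeline updates offset the cage from that location, destroy the trigger capsule and start a short delay that restores walk speed.
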(event `self.ReceiveActorBeginOverlap`
  (params (OtherActor :type "Actor Object Reference"))
  ;[1 1 1] When the trap is triggered, set the trap location
  (set `self.TrapLocation` (`SceneComponent.K2_GetComponentLocation` (`self.Cage`)))
  ;[1 1 1] Cast to the players movement, set the walk speed to 0. Only do it once to avoid bugs.
  (bind _asthird_person_character (cast `/Game/ThirdPersonBP/Blueprints/ThirdPersonCharacter` (`GameplayStatics.GetPlayerCharacter` 0)))
  (`/Engine/EditorBlueprintResources/StandardMacros.DoOnce` false
    (:`Completed`
      (bind _charactermovement (`Character.CharacterMovement` _asthird_person_character))
      (set `CharacterMovementComponent.MaxWalkSpeed` 0.0 _charactermovement)
      ;[1 1 1] Timeline for the falling trap, add this to the location and set the new world location
      (bind (_direction _newtrack_0) (`Timeline|TrapFalling`)
        (:`Update`
          (`SceneComponent.K2_SetWorldLocation` (`self.Cage`) (+ _newtrack_0 (`self.TrapLocation`)) false false)
          ;[1 1 1] Destroy the trigger, to avoid bugs
          (`ActorComponent.K2_DestroyComponent` (`self.Capsule`))
          ;[1 1 1] Delay by 0.5 then reset walk speed
          (`KismetSystemLibrary.Delay` 0.5)
          (set `CharacterMovementComponent.MaxWalkSpeed` 600.0 _charactermovement))))))

(fn `UserConstructionScript`)