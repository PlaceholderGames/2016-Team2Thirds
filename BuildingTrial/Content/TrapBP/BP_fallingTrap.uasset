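; Falling cage trap that briefly pins the player when its trigger is overlapped.
; Any actor overlap fires it once via DoOnce, zeroing player 0's ThirdPersonCharacter walk speed.
; A timeline offsets the cage from its stored world location to animate the fall.
; Timeline updates destroy the capsule trigger and run a half-second delay that restores a hardcoded walk speed.
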(event `self.ReceiveActorBeginOverlap`
  (params (OtherActor :type "Actor Object Reference"))
  ;[1 1 1] When the player triggers the trap, set it's location
  (set `self.TrapLocation` (`SceneComponent.K2_GetComponentLocation` (`self.Cage`)))
  ;[1 1 1] Cast to the players movement, change the players walk speed to 0. Only do it once.
  (bind _asthird_person_character (cast `/Game/ThirdPersonBP/Blueprints/ThirdPersonCharacter` (`GameplayStatics.GetPlayerCharacter` 0)))
  (`/Engine/EditorBlueprintResources/StandardMacros.DoOnce` false
    (:`Completed`
      (bind _charactermovement (`Character.CharacterMovement` _asthird_person_character))
      (set `CharacterMovementComponent.MaxWalkSpeed` 0.0 _charactermovement)
      ;[1 1 1] Timeline of the cage falling, then set the new location of the trap
      (bind (_direction _newtrack_0) (`Timeline|TrapFalling`)
        (:`Update`
          (`SceneComponent.K2_SetWorldLocation` (`self.Cage`) (+ _newtrack_0 (`self.TrapLocation`)) false false)
          ;[1 1 1] Destroy the trigger to avoid bugs
          (`ActorComponent.K2_DestroyComponent` (`self.Capsule`))
          ;[1 1 1] Delay by 0.5, then reset the players walk speed.
          (`KismetSystemLibrary.Delay` 0.5)
          (set `CharacterMovementComponent.MaxWalkSpeed` 600.0 _charactermovement))))))

(fn `UserConstructionScript`)