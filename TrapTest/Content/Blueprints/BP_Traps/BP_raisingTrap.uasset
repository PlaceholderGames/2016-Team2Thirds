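; BP_raisingTrap is a trap actor that moves a cage when any actor overlaps it.
; BeginPlay caches the Cage's world location, and the overlap plays the TrapFalling timeline, whose track offsets the Cage from that cached position without sweeping.
; The timeline update also destroys the Capsule component.
; The overlap has no actor filter, and a ToggleVisibility call is left unconnected.
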(event `self.ReceiveActorBeginOverlap`
  (params (OtherActor :type "Actor Object Reference"))
  (bind (_direction _newtrack_0) (`Timeline|TrapFalling`)
    (:`Update`
      (`SceneComponent.K2_SetWorldLocation` (`self.Cage`) (+ _newtrack_0 (`self.TrapLocation`)) false false)
      (`ActorComponent.K2_DestroyComponent` (`self.Capsule`)))))

(event `self.ReceiveBeginPlay`
  (set `self.TrapLocation` (`SceneComponent.K2_GetComponentLocation` (`self.Cage`))))

(fn `UserConstructionScript`)