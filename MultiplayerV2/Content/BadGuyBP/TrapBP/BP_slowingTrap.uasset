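; BP_slowingTrap is a trap that temporarily slows the player's GoodGuy character.
; Any actor overlap stores the capsule's location, then casts player character 0 to GoodGuy without checking which actor overlapped.
; It drops that character's walk speed, then restores a hardcoded normal speed after a short delay.
; The construction script sets the trap's cost.
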(event `self.ReceiveActorBeginOverlap`
  (params (OtherActor :type "Actor Object Reference"))
  ;[1 1 1] When the trap is triggered, set the trap location
  (set `self.TrapLocation` (`SceneComponent.K2_GetComponentLocation` (`self.Capsule`)))
  ;[1 1 1] Cast to the players movement, set the walk speed to 100
  (bind _asgood_guy (cast `/Game/ThirdPersonBP/Blueprints/GoodGuy` (`GameplayStatics.GetPlayerCharacter` 0)))
  (bind _charactermovement (`Character.CharacterMovement` _asgood_guy))
  (set `CharacterMovementComponent.MaxWalkSpeed` 100.0 _charactermovement)
  ;[1 1 1] Delay by 3, then reset the max speed
  (`KismetSystemLibrary.Delay` 3.0)
  (set `CharacterMovementComponent.MaxWalkSpeed` 600.0 _charactermovement))

(fn `UserConstructionScript`
  (set `self.TrapCost` 25))