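; Drain trap actor that immobilizes the player and empties their power when an actor overlaps it.
; On overlap it stores the capsule's location in TrapLocation, then casts player character 0 to GoodGuy without checking which actor overlapped.
; It zeroes walk speed and CurrentPower, prints a message, then restores a hard-coded walk speed after a short delay; power is not restored.
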(event `self.ReceiveActorBeginOverlap`
  (params (OtherActor :type "Actor Object Reference"))
  ;[1 1 1] When the trap is triggered, set the trap location
  (set `self.TrapLocation` (`SceneComponent.K2_GetComponentLocation` (`self.Capsule`)))
  ;[1 1 1] Cast to the players movement, set the walk speed to 0
  (bind _asgood_guy (cast `/Game/ThirdPersonBP/Blueprints/GoodGuy` (`GameplayStatics.GetPlayerCharacter` 0)))
  (bind _charactermovement (`Character.CharacterMovement` _asgood_guy))
  (set `CharacterMovementComponent.MaxWalkSpeed` 0.0 _charactermovement)
  ;[1 1 1] Cast to Good Guy, set current power to 0 and print string
  (bind _asgood_guy_2 (cast `/Game/ThirdPersonBP/Blueprints/GoodGuy` (`GameplayStatics.GetPlayerCharacter` 0)))
  (set `/Game/ThirdPersonBP/Blueprints/GoodGuy.CurrentPower` 0.0 _asgood_guy_2)
  (`KismetSystemLibrary.PrintString` "Your Power has been drained." true true (struct :`A` 1.0) 3.0)
  ;[1 1 1] Delay by 3, then set the walk speed back to normal
  (`KismetSystemLibrary.Delay` 3.0)
  (set `CharacterMovementComponent.MaxWalkSpeed` 600.0 _charactermovement))

(fn `UserConstructionScript`)