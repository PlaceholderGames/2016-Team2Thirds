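; Blind trap that temporarily slows the GoodGuy player and blinds them by collapsing their camera's aspect ratio to zero.
; Any overlap stores the capsule's location and affects player 0 without checking which actor overlapped.
; After a two-second delay it restores fixed walk speed and aspect ratio values rather than the previous ones.
; The construction script sets the trap's cost.
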(event `self.ReceiveActorBeginOverlap`
  (params (OtherActor :type "Actor Object Reference"))
  (bind _returnvalue (`GameplayStatics.GetPlayerCharacter` 0))
  ;[1 1 1] When the trap is triggered, set the trap location
  (set `self.TrapLocation` (`SceneComponent.K2_GetComponentLocation` (`self.Capsule`)))
  ;[1 1 1] Cast to the players movement, set the walk speed to 100
  (bind _asgood_guy (cast `/Game/ThirdPersonBP/Blueprints/GoodGuy` _returnvalue))
  (bind _charactermovement (`Character.CharacterMovement` _asgood_guy))
  (set `CharacterMovementComponent.MaxWalkSpeed` 100.0 _charactermovement)
  (bind _asgood_guy_2 (cast `/Game/ThirdPersonBP/Blueprints/GoodGuy` _returnvalue))
  (bind _camera (`/Game/ThirdPersonBP/Blueprints/GoodGuy.Camera` _asgood_guy_2))
  (`CameraComponent.SetAspectRatio` _camera 0.0)
  ;[1 1 1] Delay by 3, then reset the max speed
  (`KismetSystemLibrary.Delay` 2.0)
  (set `CharacterMovementComponent.MaxWalkSpeed` 600.0 _charactermovement)
  (`CameraComponent.SetAspectRatio` _camera 1.777778))

(fn `UserConstructionScript`
  (set `self.TrapCost` 25))